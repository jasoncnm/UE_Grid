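; BP_Pawn is a player camera pawn that pans, rotates and zooms with smoothed motion.
; Axis inputs shift a desired location along the actor's forward and right vectors and a clamped desired spring arm length, while rotation actions step a desired yaw.
; Tick interpolates the actor transform and arm length toward those targets.
; BeginPlay is empty, as the nodes seeding targets from the current state are left unconnected.
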(event `self.ReceiveBeginPlay`
  ;[1 1 1] Initialize ZoomDesired and Rotation Desired and Location Desired
)

(event `self.ReceiveTick`
  (params (DeltaSeconds :type "Float (single-precision)"))
  (bind _springarm (`self.SpringArm`))
  ;[1 1 1] Set Camera Rotation, Location, ArmLength
  (set `SpringArmComponent.TargetArmLength` (`KismetMathLibrary.FInterpTo` (`SpringArmComponent.TargetArmLength` _springarm) (`self.Zoom_Desired`) DeltaSeconds (`self.Zoom Interp`)) _springarm)
  (`self.K2_SetActorLocation` (`KismetMathLibrary.VInterpTo` (`self.K2_GetActorLocation`) (`self.Location_Desired`) DeltaSeconds (`self.Location Interp`)))
  (`self.K2_SetActorRotation` (`KismetMathLibrary.RInterpTo` (`self.K2_GetActorRotation`) (`self.Rotation_Desired`) DeltaSeconds (`self.Rotation Interp`))))

(event `InputAxis|InputAxis_Camera_Zoom`
  (params (AxisValue :type "Float (single-precision)"))
  ;[1 1 1] Set Zoom Desired
  (set `self.Zoom_Desired` (`KismetMathLibrary.FClamp` (+ (* AxisValue (`self.Zoom Speed`)) (`self.Zoom_Desired`)) (`self.Zoom Min`) (`self.Zoom Max`))))

(event `InputAxis|InputAxis_Camera_Forward`
  (params (AxisValue :type "Float (single-precision)"))
  ;[1 1 1] Set Location Desired
  (set `self.Location_Desired` (+ (`self.Location_Desired`) (* (* AxisValue (`self.Location Speed`)) (`self.GetActorForwardVector`)))))

(event `InputAxis|InputAxis_Camera_Right`
  (params (AxisValue :type "Float (single-precision)"))
  ;[1 1 1] Set Location Desired
  (set `self.Location_Desired` (+ (`self.Location_Desired`) (* (* AxisValue (`self.Location Speed`)) (`self.GetActorRightVector`)))))

(event `InputAction|InputAction_Rotaiton_Right`
  (params (Key :type "Key Structure"))
  ;[1 1 1] Set Rotation Desired
  (:`Pressed`
    (set `self.Rotation_Desired` (`KismetMathLibrary.ComposeRotators` (`self.Rotation_Desired`) (`KismetMathLibrary.MakeRotator` 0.0 0.0 (- 0.0 (`self.Rotation Speed`)))))))

(event `InputAction|InputAction_Rotation_Left`
  (params (Key :type "Key Structure"))
  ;[1 1 1] Set Rotation Desired
  (:`Pressed`
    (set `self.Rotation_Desired` (`KismetMathLibrary.ComposeRotators` (`self.Rotation_Desired`) (`KismetMathLibrary.MakeRotator` 0.0 0.0 (`self.Rotation Speed`))))))

(fn `UserConstructionScript`)