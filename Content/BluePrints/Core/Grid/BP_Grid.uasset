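; BP_Grid builds a tile grid of squares, hexagons or triangles as instances of one InstancedStaticMesh.
; SpawnGrid clears old instances, applies mesh and material from DT_CreatShapeData, then derives a snapped center and bottom-left origin.
; Per-shape spacing places each tile, with hexagons using doubled, parity-offset Y indices and triangles flipping yaw by index parity.
; The construction script's SpawnGrid call is disconnected, so nothing here triggers a build.
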(fn `CalculateCenterAndBottomLeft`
  (returns (Center :type "Vector Structure") (BottomLeft :type "Vector Structure"))
  (locals (C :type "Vector Structure" :default (0.0 0.0 0.0)))
  (bind (_grid_tile_count_x _grid_tile_count_y) (`KismetMathLibrary.BreakVector2D` (`self.Grid Tile Count`)))
  (bind (_returnvalue_x _returnvalue_y) (`KismetMathLibrary.BreakVector2D` (* (/ (`self.Grid Tile Count`) (3.0 2.0)) (`KismetMathLibrary.Conv_VectorToVector2D` (`self.Grid Tile Size`)))))
  (bind (_returnvalue_x_2 _returnvalue_y_2) (`KismetMathLibrary.BreakVector2D` (* (/ (- (`self.Grid Tile Count`) (1.0 1.0)) (2.0 4.0)) (`KismetMathLibrary.Conv_VectorToVector2D` (`self.Grid Tile Size`)))))
  (bind (_returnvalue_x_3 _returnvalue_y_3) (`KismetMathLibrary.BreakVector2D` (* (/ (- (`self.Grid Tile Count`) (`KismetMathLibrary.MakeVector2D` (`KismetMathLibrary.SelectFloat` 0.0 1.0 (`/Game/BluePrints/Core/Utilities/BFL_Utilities.IsFloatEven` _grid_tile_count_x)) (`KismetMathLibrary.SelectFloat` 0.0 1.0 (`/Game/BluePrints/Core/Utilities/BFL_Utilities.IsFloatEven` _grid_tile_count_y)))) 2.0) (`KismetMathLibrary.Conv_VectorToVector2D` (`self.Grid Tile Size`)))))
  (switch `/Game/BluePrints/Core/Grid/Grid_Shpes/E_GridShape` (`self.Grid Shape`)
    (:`NewEnumerator1`
      (set `local.C` (`/Game/BluePrints/Core/Utilities/BFL_Utilities.Snap Vector to Vector` (`self.Grid Center Location`) (`self.Grid Tile Size`)))
      (return (`local.C`) (- (`local.C`) (`KismetMathLibrary.MakeVector` _returnvalue_x_3 _returnvalue_y_3))))
    (:`NewEnumerator2`
      (set `local.C` (`/Game/BluePrints/Core/Utilities/BFL_Utilities.Snap Vector to Vector` (`self.Grid Center Location`) (* (`self.Grid Tile Size`) (1.5 1.0 1.0))))
      (return (`local.C`) (- (`local.C`) (`/Game/BluePrints/Core/Utilities/BFL_Utilities.Snap Vector to Vector` (`KismetMathLibrary.MakeVector` _returnvalue_x _returnvalue_y) (* (`self.Grid Tile Size`) (1.5 1.0 1.0))))))
    (:`NewEnumerator3`
      (set `local.C` (`/Game/BluePrints/Core/Utilities/BFL_Utilities.Snap Vector to Vector` (`self.Grid Center Location`) (* (`self.Grid Tile Size`) (2.0 1.0 1.0))))
      (return (`local.C`) (- (`local.C`) (`/Game/BluePrints/Core/Utilities/BFL_Utilities.Snap Vector to Vector` (`KismetMathLibrary.MakeVector` _returnvalue_x_2 _returnvalue_y_2) (* (`self.Grid Tile Size`) (2.0 1.0 1.0))))))))

(fn `DestroyGrid`
  (`InstancedStaticMeshComponent.ClearInstances` (`self.InstancedStaticMesh`)))

(fn `Get Current Shape Data`
  (returns (ReturnValue :type "/Game/BluePrints/Core/Grid/Grid_Shpes/S_GridShape_Data Structure"))
  (bind _returnvalue (`|GetEnumeratorNameAsString` (`self.Grid Shape`)))
  (bind _returnvalue_2 (`|GetDataTableRow` "/Game/BluePrints/Core/Grid/Grid_Shpes/DT_CreatShapeData.DT_CreatShapeData" (`KismetStringLibrary.Conv_StringToName` _returnvalue))
    (:`then`
      _)
    (:`RowNotFound`
      (`KismetSystemLibrary.PrintString` (`KismetStringLibrary.Concat_StrStr` "ERROR - Row Not Found " _returnvalue) true true (struct :`R` 1.0 :`A` 1.0) 5.0)))
  (return _returnvalue_2))

(fn `Get Tile Location from Grid Index`
  (params (Index :type "Vector2D Structure"))
  (returns (Location :type "Vector Structure"))
  (bind (_returnvalue_x _returnvalue_y) (`KismetMathLibrary.BreakVector2D` (* Index (select `/Game/BluePrints/Core/Grid/Grid_Shpes/E_GridShape` (`self.Grid Shape`) :`NewEnumerator1` (1.0 1.0) :`NewEnumerator2` (0.75 0.5) :`NewEnumerator3` (1.0 0.5) :!type "Vector2D Structure"))))
  (return (+ (`self.GridButtomLeftLoc`) (* (`self.Grid Tile Size`) (`KismetMathLibrary.MakeVector` _returnvalue_x _returnvalue_y)))))

(fn `Get TIle Rotation from Grid Index`
  (params (GridIndex :type "Vector2D Structure"))
  (returns (TileRotation :type "Rotator Structure"))
  (bind (_gridindex_x _gridindex_y) (`KismetMathLibrary.BreakVector2D` (`local.GridIndex`)))
  (if (`|EnumEquality` (`self.Grid Shape`) "NewEnumerator3")
    (return (`KismetMathLibrary.MakeRotator` 0.0 0.0 (+ (`KismetMathLibrary.SelectFloat` 180.0 0.0 (`/Game/BluePrints/Core/Utilities/BFL_Utilities.IsFloatEven` _gridindex_x)) (`KismetMathLibrary.SelectFloat` 180.0 0.0 (`/Game/BluePrints/Core/Utilities/BFL_Utilities.IsFloatEven` _gridindex_y)))))
    (else
      (return))))

(fn `SpawnGrid`
  (params (CenterLocation :type "Vector Structure") (TileSize :type "Vector Structure") (TileCount :type "Vector2D Structure") (Shape :type "/Game/BluePrints/Core/Grid/Grid_Shpes/E_GridShape Enum" :default "NewEnumerator0"))
  (locals (X :type Integer) (Y :type Integer) (TileTransform :type "Transform Structure") (Index :type "Vector2D Structure"))
  (bind _instancedstaticmesh (`self.InstancedStaticMesh`))
  (bind (_tilecount_x _tilecount_y) (`KismetMathLibrary.BreakVector2D` (`local.TileCount`)))
  (bind (_grid_tile_count_x _grid_tile_count_y) (`KismetMathLibrary.BreakVector2D` (`self.Grid Tile Count`)))
  (bind (_grid_tile_count_x_2 _grid_tile_count_y_2) (`KismetMathLibrary.BreakVector2D` (`self.Grid Tile Count`)))
  (bind _grid_tile_count_x_3 (`KismetMathLibrary.BreakVector2D` (`self.Grid Tile Count`)))
  (bind (_meshsize _mesh _meshmaterial _flatmesh _flatbordermaterial) (break `/Game/BluePrints/Core/Grid/Grid_Shpes/S_GridShape_Data` (`self.Get Current Shape Data`)))
  (set `self.Grid Center Location` CenterLocation)
  (set `self.Grid Tile Size` TileSize)
  (set `self.Grid Shape` Shape)
  (set `self.Grid Tile Count` (`KismetMathLibrary.MakeVector2D` (`KismetMathLibrary.Conv_IntToDouble` (`KismetMathLibrary.Round` _tilecount_x)) (`KismetMathLibrary.Conv_IntToDouble` (`KismetMathLibrary.Round` _tilecount_y))))
  (`self.DestroyGrid`)
  (`StaticMeshComponent.SetStaticMesh` _instancedstaticmesh _flatmesh)
  (`PrimitiveComponent.SetMaterial` _instancedstaticmesh 0 _flatbordermaterial)
  (bind (_center _bottomleft) (`self.CalculateCenterAndBottomLeft`))
  (set `self.Grid Center Location` _center)
  (set `self.GridButtomLeftLoc` _bottomleft)
  (for _index (range (`KismetMathLibrary.Round` _grid_tile_count_x_3))
    (set `local.X` _index)
    (if (`|EnumInequality` (`self.Grid Shape`) "NewEnumerator2")
      (for _index_2 (range (`KismetMathLibrary.Round` _grid_tile_count_y))
        (set `local.Y` _index_2)
        (set `local.Index` (`KismetMathLibrary.MakeVector2D` (`KismetMathLibrary.Conv_IntToDouble` (`local.X`)) (`KismetMathLibrary.Conv_IntToDouble` (`local.Y`))) :!label _label)
        (set `local.TileTransform` (`KismetMathLibrary.MakeTransform` (+ (`self.Get Tile Location from Grid Index` (`local.Index`)) (0.0 0.0 2.0)) (`self.Get TIle Rotation from Grid Index` (`local.Index`)) (/ (`self.Grid Tile Size`) (`.MeshSize_2_4FBC98284DB2FB1FCA24608AC4C70A59` (break `/Game/BluePrints/Core/Grid/Grid_Shpes/S_GridShape_Data` (`self.Get Current Shape Data`))))))
        (`InstancedStaticMeshComponent.AddInstance` (`self.InstancedStaticMesh`) (`local.TileTransform`) true))
      (else
        (for _index_3 (range (`KismetMathLibrary.SelectInt` 0 1 (`/Game/BluePrints/Core/Utilities/BFL_Utilities.IsIntEven` (`local.X`))) (* (`KismetMathLibrary.Round` _grid_tile_count_y_2) 2))
          (set `local.Y` _index_3)
          (`|ExecutionSequence`
            (:`then_0`
              (goto _label))
            (:`then_1`
              (`/Engine/EditorBlueprintResources/StandardMacros.IncrementInt` _index_3))))))))

(fn `UserConstructionScript`)